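; BP_Semafor_Chodci is a pedestrian traffic light for a crossroads that alternates between two states on its own timer.
; Tick runs a five-second Delay, then advances State, wraps it to zero and fires ChangeState, which BeginPlay also calls for the initial state.
; ChangeLightState reads the state's LightStates integer as decimal digit flags: units show the Green component, tens show Red.
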(event Custom|Event%20ChangeState
  (CallFunction|ChangeLightState (Variables|Default|GetState) (Variables|Default|GetLightStates)))

(event EventBeginPlay
  (CallFunction|EventChangeState))

(event Collision|EventActorBeginOverlap
  (params (OtherActor :type Actor%20Object%20Reference)))

(event EventTick
  (params (DeltaSeconds :type Float%20%28single-precision%29))
  (Utilities|FlowControl|Delay 5.0)
  (bind _result (Math|Integer|IncrementInt (Variables|Default|GetState))
    (:%20%20
      (if (== _result 2)
        (Variables|Default|SetState 0)
        (else
          (Variables|Default|SetState _result)))
      (CallFunction|EventChangeState))))

(fn ConstructionScript)

(fn ChangeLightState
  (params (Dimension%201 :type Integer) (Array :type Array%20of%20Bytes))
  (bind _output (Utilities|Array|Get(acopy) Array Dimension%201))
  (Rendering|SetVisibility (Variables|Default|GetGreen) (== (Class|KismetMathLibrary|PercentByteByte _output 10) 1) false)
  (Rendering|SetVisibility (Variables|Default|GetRed) (== (Class|KismetMathLibrary|PercentByteByte (/ _output 10) 10) 1) false))