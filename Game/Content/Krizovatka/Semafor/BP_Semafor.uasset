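; Traffic light actor for an intersection that cycles through four states, with its body variant chosen by SemaforType in the construction script.
; A Delay on Tick advances State roughly every second, wrapping to zero, and fires ChangeState.
; ChangeLightState decodes the LightStates entry digit by digit (hundreds red, tens yellow, ones green) to toggle visibility of child components tagged red, yel or green.
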(event Custom|Event%20ChangeState
  (CallFunction|ChangeLightState (Variables|Default|GetState) (Variables|Default|GetLightStates)))

(event EventBeginPlay
  (CallFunction|EventChangeState))

(event Collision|EventActorBeginOverlap
  (params (OtherActor :type Actor%20Object%20Reference)))

(event EventTick
  (params (DeltaSeconds :type Float%20%28single-precision%29))
  (Utilities|FlowControl|Delay 1.0)
  (bind _result (Math|Integer|IncrementInt (Variables|Default|GetState))
    (:%20%20
      (if (== _result 4)
        (Variables|Default|SetState 0)
        (else
          (Variables|Default|SetState _result)))
      (CallFunction|EventChangeState))))

(fn ConstructionScript
  (bind _semafortype (Variables|Default|GetSemaforType))
  (Rendering|SetVisibility (Variables|Default|GetBOne) (Utilities|Enum|Equal(Enum) _semafortype "NewEnumerator0") true)
  (Rendering|SetVisibility (Variables|Default|GetBTwo) (Utilities|Enum|Equal(Enum) _semafortype "NewEnumerator1") true)
  (Rendering|SetVisibility (Variables|Default|Getsmall) (Utilities|Enum|Equal(Enum) _semafortype "NewEnumerator2") true))

(fn ChangeLightState
  (params (Dimension%201 :type Integer) (Array :type Array%20of%20Bytes))
  (bind _output (Utilities|Array|Get(acopy) Array Dimension%201))
  (bind _returnvalue (/ _output 10))
  (for _array_element (Components|GetChildrenComponents (Variables|Default|GetDefaultSceneRoot) true)
    (if (Components|ComponentHasTag _array_element "green")
      (Rendering|SetVisibility _array_element (== (Class|KismetMathLibrary|PercentByteByte _output 10) 1) false)
      (elif (Components|ComponentHasTag _array_element "yel")
        (Rendering|SetVisibility _array_element (== (Class|KismetMathLibrary|PercentByteByte _returnvalue 10) 1) false)
        (elif (Components|ComponentHasTag _array_element "red")
          (Rendering|SetVisibility _array_element (== (Class|KismetMathLibrary|PercentByteByte (/ _returnvalue 10) 10) 1) false))))))