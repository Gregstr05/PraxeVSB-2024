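; Push-button Blueprint for a traffic light at an intersection, apparently an unfinished pedestrian crossing request.
; PushButton passes a DoOnce, prints a debug message, then loops over the Auta (cars) and Chodci (pedestrians) arrays checking each element's State.
; Both state checks have empty branches, a short trailing Delay leads nowhere, and nothing resets the DoOnce.
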(event EventBeginPlay)

(event Collision|EventActorBeginOverlap
  (params (OtherActor :type Actor%20Object%20Reference)))

(event EventTick
  (params (DeltaSeconds :type Float%20%28single-precision%29)))

(event EventPushButton
  (Utilities|FlowControl|DoOnce false
    (:Completed
      (Development|PrintString "Button pressed")
      (for _array_element (Variables|Default|GetAuta)
        (if (== (Variables|/Game/Krizovatka/Semafor/BP_Semafor.BP_Semafor_C|GetState _array_element) 0)
          _))
      (for _array_element_2 (Variables|Default|GetChodci)
        (if (== (Variables|/Game/Krizovatka/Semafor/BP_Semafor_Chodci.BP_Semafor_Chodci_C|GetState _array_element_2) 1)
          _))
      (Utilities|FlowControl|Delay 0.2))))

(fn ConstructionScript)