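; Snap point for the prop system that decides whether a prop can snap onto its SnapCol component.
; The construction script writes SnapParam into SnapCol's component tags.
; TrySnap requires a matching tag and a per-axis rotation difference within Tolerance, then messages the parent actor and returns SnapCol.
; Tolerance is exposed through a getter, while Detach and SendParams return only empty defaults.
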(event EventBeginPlay)

(event Collision|EventActorBeginOverlap
  (params (OtherActor :type Actor%20Object%20Reference)))

(event EventTick
  (params (DeltaSeconds :type Float%20%28single-precision%29)))

(fn ConstructionScript
  (Utilities|Array|SetArrayElem (Variables|/Script/Engine.ActorComponent|GetComponentTags (Variables|Default|GetSnapCol)) 0 (Variables|Default|GetSnapParam) true))

(fn De-tach
  (params (bAttach :type Boolean) (AttachTo :type Scene%20Component%20Object%20Reference))
  (return false))

(fn SendParams
  (params (bIn :type Boolean) (NameIn :type Name :default "None") (VecIn :type Vector :default "0, 0, 0") (SC_In :type Scene%20Component%20Object%20Reference) (Actor :type Actor%20Object%20Reference))
  (return false "None" "0, 0, 0" 0 0.0))

(fn SendPropSnapTolerance
  (return (Variables|Default|GetTolerance)))

(fn TrySnap
  (params (PropAllign :type Scene%20Component%20Object%20Reference))
  (bind _returnvalue (Transformation|GetWorldRotation PropAllign))
  (bind _snapcol (Variables|Default|GetSnapCol))
  (bind _tolerance (Variables|Default|GetTolerance))
  (bind _returnvalue_2 (Transformation|GetWorldRotation _snapcol))
  (bind _componenttags (Variables|/Script/Engine.ActorComponent|GetComponentTags _snapcol))
  (bind _returnvalue_3 (Class|KismetMathLibrary|NegateRotator _returnvalue_2))
  (bind _output (Utilities|Array|Get(acopy) _componenttags))
  (bind _returnvalue_4 (Math|Rotator|CombineRotators _returnvalue _returnvalue_3))
  (if (Components|ComponentHasTag PropAllign _output)
    (if (Math|Boolean|ANDBoolean (< (Math|Float|Absolute(Float) (.roll _returnvalue_4)) (.x _tolerance)) (< (Math|Float|Absolute(Float) (.pitch _returnvalue_4)) (.y _tolerance)) (< (Math|Float|Absolute(Float) (.yaw _returnvalue_4)) (.z _tolerance)))
      (Class|BPIInteractions|SnapInteract(Message) (Actor|GetParentActor) _output)
      (return true (Variables|Default|GetSnapCol))
      (else
        _)))
  (return false 0))