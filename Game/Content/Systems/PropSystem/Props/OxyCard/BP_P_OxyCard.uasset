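; BP_P_OxyCard is a snappable card prop in the prop system, with a color variant and a widget screen.
; The construction script picks one of five card materials from the second component tag on Allign.
; When snapped, it shows the widget, fills it with card data requested from the interacting actor, and registers itself there; unsnapping hides and clears.
; AMSSendParam messages are forwarded to the widget.
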(event EventBeginPlay
  (|CallParentFunction) ; This node is disabled and will not be called.\nDrag off pins to build functionality.
)

(event Collision|EventActorBeginOverlap
  (params (OtherActor :type Actor%20Object%20Reference))
  (|CallParentFunction OtherActor) ; This node is disabled and will not be called.\nDrag off pins to build functionality.
)

(event EventTick
  (params (DeltaSeconds :type Float%20%28single-precision%29))
  (|CallParentFunction DeltaSeconds) ; This node is disabled and will not be called.\nDrag off pins to build functionality.
)

(event EventAMSSendParam
  (params (BoolParam :type Boolean) (NameParam :type Name :default "None"))
  (Class|BPIInteractions|AMSSendParam(Message) (UserInterface|GetWidget (Variables|Default|GetWidget)) BoolParam NameParam))

(fn ConstructionScript
  (bind _allign (Variables|Default|GetAllign))
  (bind _staticmesh (Variables|Default|GetStaticMesh))
  (bind _componenttags (Variables|/Script/Engine.ActorComponent|GetComponentTags _allign))
  (bind _output (Utilities|Array|Get(acopy) _componenttags 1))
  (|CallParentFunction)
  (Utilities|IfName _output "R"
    (:True
      (Rendering|Material|SetMaterial _staticmesh 0 "/Game/Systems/PropSystem/Props/OxyCard/MI_card_R.MI_card_R"))
    (:False
      (Utilities|IfName _output "G"
        (:True
          (Rendering|Material|SetMaterial _staticmesh 0 "/Game/Systems/PropSystem/Props/OxyCard/MI_card_G.MI_card_G"))
        (:False
          (Utilities|IfName _output "B"
            (:True
              (Rendering|Material|SetMaterial _staticmesh 0 "/Game/Systems/PropSystem/Props/OxyCard/MI_card_B.MI_card_B"))
            (:False
              (Utilities|IfName _output "Y"
                (:True
                  (Rendering|Material|SetMaterial _staticmesh 0 "/Game/Systems/PropSystem/Props/OxyCard/MI_card_Y.MI_card_Y"))
                (:False
                  (Utilities|IfName _output "C"
                    (:True
                      (Rendering|Material|SetMaterial _staticmesh 0 "/Game/Systems/PropSystem/Props/OxyCard/MI_card_C.MI_card_C"))))))))))))

(fn OnSnap
  (params (bSnapped :type Boolean) (IA :type Actor%20Object%20Reference))
  (Rendering|SetVisibility (Variables|Default|GetWidget) bSnapped false)
  (if bSnapped
    (bind _knobvals (Class|BPIOxyCom|SendCardData(Message) IA (Utilities|Array|Get(acopy) (Variables|Default|GetSnapParams) 1)))
    (Class|BPIOxyCom|SetWidgetScreen(Message) (UserInterface|GetWidget (Variables|Default|GetWidget)) _knobvals)
    (Class|BPIInterInit|SetActor(Message) IA self "None")
    (else
      (Class|BPIInterInit|SetActor(Message) IA 0 "None"))))

(fn SendCardData
  (params (KnobsParam :type Name :default "None"))
  (return 0))