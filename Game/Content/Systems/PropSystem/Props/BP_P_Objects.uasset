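; BP_P_Objects is a prop Blueprint in the prop system that represents assorted small household objects, such as kitchenware, tools and toiletries, through one configurable actor.
; After running the parent construction script, it picks the static mesh from the Type selection.
; It then moves the Allign component to the AllighnOffset relative location.
; The event graph adds no logic of its own.
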(event EventBeginPlay
  (|CallParentFunction) ; This node is disabled and will not be called.\nDrag off pins to build functionality.
)

(event Collision|EventActorBeginOverlap
  (params (OtherActor :type Actor%20Object%20Reference))
  (|CallParentFunction OtherActor) ; This node is disabled and will not be called.\nDrag off pins to build functionality.
)

(event EventTick
  (params (DeltaSeconds :type Float%20%28single-precision%29))
  (|CallParentFunction DeltaSeconds) ; This node is disabled and will not be called.\nDrag off pins to build functionality.
)

(fn ConstructionScript
  (|CallParentFunction)
  (Components|StaticMesh|SetStaticMesh (Variables|Default|GetStaticMesh) (Utilities|Select :Index (Variables|Default|GetType) :NewEnumerator0 "/Game/Meshes/pan.pan" :NewEnumerator1 "/Game/Meshes/TinCan.TinCan" :NewEnumerator2 "/Game/Meshes/kettle.kettle" :NewEnumerator3 "/Game/Meshes/pillow.pillow" :NewEnumerator4 "/Game/Meshes/vYno.vYno" :NewEnumerator5 "/Game/Meshes/tools/drill.drill" :NewEnumerator6 "/Game/Meshes/tools/hammer.hammer" :NewEnumerator7 "/Game/Meshes/tools/pliers.pliers" :NewEnumerator8 "/Game/Meshes/tools/saw.saw" :NewEnumerator9 "/Game/Meshes/tools/screwdriver.screwdriver" :NewEnumerator10 "/Game/Meshes/tools/wrench.wrench" :NewEnumerator11 "/Game/Meshes/hygiena/kartacek.kartacek" :NewEnumerator12 "/Game/Meshes/hygiena/mydlo.mydlo" :NewEnumerator13 "/Game/Meshes/hygiena/pasta.pasta" :NewEnumerator14 "/Game/Meshes/hygiena/samponek.samponek" :NewEnumerator15 "/Game/Meshes/SM_can.SM_can" :NewEnumerator17 "/Game/Meshes/pot.pot" :NewEnumerator18 "/Game/Meshes/mug.mug"))
  (Transformation|SetRelativeLocation (Variables|Default|GetAllign) (Variables|Default|GetAllighnOffset) false true))