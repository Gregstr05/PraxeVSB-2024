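; Keycard prop with a configurable card color that can start frozen, covered by the Led (ice) mesh.
; Construction applies the color through a dynamic material and shows the Led mesh only when frozen.
; While frozen, its fourth StaticMesh component tag is nulled, with SMParams[0] saved for later.
; An "Unfreeze" interaction plays a scale timeline on Led, then hides it, disables its collision and restores the tag.
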(event EventBeginPlay
  (bind _bfreezed (Variables|Default|GetbFreezed))
  (|CallParentFunction)
  (if _bfreezed
    (Variables|Default|SetParamIfFreeezed (Utilities|Array|Get(acopy) (Variables|Default|GetSM_Params)))
    (Utilities|Array|SetArrayElem (Variables|/Script/Engine.ActorComponent|GetComponentTags (Variables|Default|GetStaticMesh)) 3 "Null" true)
    (Collision|SetCollisionEnabled (Variables|Default|Getled) (select _bfreezed "QueryAndPhysics" "NoCollision"))))

(event Collision|EventActorBeginOverlap
  (params (OtherActor :type Actor%20Object%20Reference))
  (|CallParentFunction OtherActor) ; This node is disabled and will not be called.\nDrag off pins to build functionality.
)

(event EventTick
  (params (DeltaSeconds :type Float%20%28single-precision%29))
  (|CallParentFunction DeltaSeconds) ; This node is disabled and will not be called.\nDrag off pins to build functionality.
)

(event EventInteract
  (params (Param :type Name :default "None"))
  (bind _led (Variables|Default|Getled))
  (Utilities|IfName Param "Unfreeze"
    (:True
      (if (Variables|Default|GetbFreezed)
        (bind _newtrack_0 (Timeline|Scale Play)
          (:Update
            (Transformation|SetWorldScale3D (Variables|Default|Getled) (* "0.072500,0.072500,0.072500" _newtrack_0)))
          (:Finished
            (Collision|SetCollisionEnabled _led "NoCollision")
            (Rendering|SetVisibility _led false false)
            (Variables|Default|SetbFreezed false)
            (Utilities|Array|SetArrayElem (Variables|/Script/Engine.ActorComponent|GetComponentTags (Variables|Default|GetStaticMesh)) 3 (Variables|Default|GetParamIfFreeezed))))))))

(fn ConstructionScript
  (bind _bfreezed (Variables|Default|GetbFreezed))
  (bind _led (Variables|Default|Getled))
  (|CallParentFunction)
  (bind _returnvalue (Rendering|Material|CreateDynamicMaterialInstance "/Game/Materials/MI_keycard.MI_keycard" "None" "None" :!class /Script/Engine.KismetMaterialLibrary))
  (Rendering|Material|SetMaterial (Variables|Default|GetStaticMesh) 0 _returnvalue)
  (Rendering|Material|SetVectorParameterValue _returnvalue "CardColor" (Variables|Default|GetCardColor) :!class /Script/Engine.MaterialInstanceDynamic)
  (Rendering|SetVisibility _led _bfreezed false)
  (Collision|SetCollisionEnabled _led (select _bfreezed "QueryAndPhysics" "NoCollision")))