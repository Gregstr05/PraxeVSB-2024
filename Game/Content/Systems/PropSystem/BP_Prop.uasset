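; Physics prop that can be picked up, dropped or snapped into matching BP_PropSnap sockets.
; Construction sets interaction and snap tags; BeginPlay caches the mesh's offset from its Allign component.
; Overlapping a tag-matched socket places a Ghost preview and enables Tick, which shows it only within rotation tolerance.
; De-tach attaches to the carrier, or on release snaps via the socket or restores physics, calling the empty OnSnap hook.
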(event OnComponentBeginOverlap(Allign)
  (params (OverlappedComponent :type Primitive%20Component%20Object%20Reference) (OtherActor :type Actor%20Object%20Reference) (OtherComp :type Primitive%20Component%20Object%20Reference) (OtherBodyIndex :type Integer) (bFromSweep :type Boolean) (SweepResult :type Hit%20Result%20Structure%20%28by%20ref%29))
  (bind _allignoffset (Variables|Default|GetAllignOffset))
  (if (Components|ComponentHasTag OtherComp (Utilities|Array|Get(acopy) (Variables|/Script/Engine.ActorComponent|GetComponentTags (Variables|Default|GetAllign))))
    (bind _tolerance (Class|BPIProps|SendPropSnapTolerance(Message) OtherActor))
    (bind _output_get (Variables|GhostDraw|SetPropSnapCol OtherComp))
    (Variables|GhostDraw|SetPropSnapTolerance _tolerance)
    (Transformation|SetWorldLocationAndRotation (Variables|Default|GetGhost) (+ (.location (Transformation|GetWorldTransform _output_get)) (Math|Vector|RotateVector (.location _allignoffset) (Math|Rotator|CombineRotators (.rotation _allignoffset) (.rotation (Transformation|GetWorldTransform _output_get))))) (Math|Rotator|CombineRotators (.rotation _allignoffset) (.rotation (Transformation|GetWorldTransform _output_get))) false true)
    (Actor|Tick|SetActorTickEnabled true)))

(event OnComponentEndOverlap(Allign)
  (params (OverlappedComponent :type Primitive%20Component%20Object%20Reference) (OtherActor :type Actor%20Object%20Reference) (OtherComp :type Primitive%20Component%20Object%20Reference) (OtherBodyIndex :type Integer))
  (if (== OtherComp (Variables|GhostDraw|GetPropSnapCol))
    (Variables|GhostDraw|SetPropSnapCol 0)
    (Actor|Tick|SetActorTickEnabled false)
    (Rendering|SetVisibility (Variables|Default|GetGhost) false false)))

(event EventBeginPlay
  (bind _staticmesh (Variables|Default|GetStaticMesh))
  (bind _returnvalue (Transformation|GetWorldRotation _staticmesh))
  (Variables|Default|SetAllignOffset (Math|Transform|MakeTransform (Math|Vector|UnrotateVector (- (Transformation|GetWorldLocation (Variables|Default|GetStaticMesh)) (Transformation|GetWorldLocation (Variables|Default|GetAllign))) _returnvalue) (Math|Rotator|CombineRotators _returnvalue (Class|KismetMathLibrary|NegateRotator (Transformation|GetWorldRotation (Variables|Default|GetAllign)))) "1.000000,1.000000,1.000000")))

(event Collision|EventActorBeginOverlap
  (params (OtherActor :type Actor%20Object%20Reference)))

(event EventTick
  (params (DeltaSeconds :type Float%20%28single-precision%29))
  (bind _propsnaptolerance (Variables|GhostDraw|GetPropSnapTolerance))
  (bind _allign (Variables|Default|GetAllign))
  (bind _propsnapcol (Variables|GhostDraw|GetPropSnapCol))
  (bind _returnvalue (Transformation|GetWorldRotation _propsnapcol))
  (bind _returnvalue_2 (Transformation|GetWorldRotation _allign))
  (bind _returnvalue_3 (Class|KismetMathLibrary|NegateRotator _returnvalue_2))
  (bind _returnvalue_4 (Math|Rotator|CombineRotators _returnvalue _returnvalue_3))
  (Rendering|SetVisibility (Variables|Default|GetGhost) (Math|Boolean|ANDBoolean (< (Math|Float|Absolute(Float) (.roll _returnvalue_4)) (.x _propsnaptolerance)) (< (Math|Float|Absolute(Float) (.pitch _returnvalue_4)) (.y _propsnaptolerance)) (< (Math|Float|Absolute(Float) (.yaw _returnvalue_4)) (.z _propsnaptolerance))) false))

(fn ConstructionScript
  (bind _ghost (Variables|Default|GetGhost))
  (Utilities|Array|SetArrayElem (Variables|/Script/Engine.ActorComponent|GetComponentTags (Variables|Default|GetStaticMesh)) 0 (Utilities|String|SelectName "Interactible" "None" (Variables|Default|GetbIsInteractible)) true)
  (Utilities|Array|SetArrayElem (Variables|/Script/Engine.ActorComponent|GetComponentTags (Variables|Default|GetStaticMesh)) 1 (Utilities|String|SelectName "Pickable" "None" (Variables|Default|GetbIsPickable)) true)
  (Utilities|Array|SetArrayElem (Variables|/Script/Engine.ActorComponent|GetComponentTags (Variables|Default|GetStaticMesh)) 2 "DynamicInteract" true)
  (for (_array_element _array_index) (Variables|Default|GetSM_Params)
    (Utilities|Array|SetArrayElem (Variables|/Script/Engine.ActorComponent|GetComponentTags (Variables|Default|GetStaticMesh)) (+ _array_index 3) _array_element true))
  (Variables|/Script/Engine.ActorComponent|SetComponentTags (Variables|Default|GetAllign) (Variables|Default|GetSnapParams))
  (Components|StaticMesh|SetStaticMesh _ghost (Variables|/Script/Engine.StaticMeshComponent|GetStaticMesh (Variables|Default|GetStaticMesh)))
  (Rendering|Material|SetMaterial _ghost 1 "/Engine/EditorResources/FieldNodes/_Resources/M_FieldRadiusPreview.M_FieldRadiusPreview"))

(fn OnSnap
  (params (bSnapped :type Boolean) (IA :type Actor%20Object%20Reference))
  (return))

(fn De-tach
  (params (bAttach :type Boolean) (AttachTo :type Scene%20Component%20Object%20Reference))
  (bind _staticmesh (Variables|Default|GetStaticMesh))
  (bind _allignoffset (Variables|Default|GetAllignOffset))
  (bind _staticmesh_2 (Variables|Default|GetStaticMesh))
  (if bAttach
    (if (not (and (Variables|Default|GetbAttached) (not (Variables|Default|GetbPickableAfterSnap))))
      (Variables|Default|SetbAttached false)
      (Physics|SetSimulatePhysics _staticmesh false)
      (Class|BPIProps|SnapDispatchCall(Message) (Variables|Default|GetPropSnap) false)
      (Variables|Default|SetPropSnap 0)
      (Transformation|AttachComponentToComponent _staticmesh AttachTo "None" "SnapToTarget" "KeepWorld" "KeepWorld" false)
      (Transformation|AddWorldOffset _staticmesh_2 (- (Transformation|GetWorldLocation _staticmesh_2) (Transformation|GetWorldLocation (Variables|Default|GetAllign))) false true)
      (CallFunction|OnSnap false :!label _label)
      (return bAttach self))
    (else
      (for _array_element (Collision|GetOverlappingActors (Variables|Default|GetAllign) "/Game/Systems/PropSystem/BP_PropSnap.BP_PropSnap_C" :!class /Script/Engine.PrimitiveComponent)
        (bind (_bsucces _propsnapcol) (Class|BPIProps|TrySnap(Message) _array_element (Variables|Default|GetAllign)))
        (if _bsucces
          (Variables|Default|SetPropSnap (Components|GetOwner _propsnapcol))
          (Transformation|AttachComponentToComponent _staticmesh _propsnapcol "None" "KeepWorld" "KeepWorld" "KeepWorld" false)
          (Transformation|SetWorldLocationAndRotation _staticmesh (+ (.location (Transformation|GetWorldTransform _propsnapcol)) (Math|Vector|RotateVector (.location _allignoffset) (Math|Rotator|CombineRotators (.rotation _allignoffset) (.rotation (Transformation|GetWorldTransform _propsnapcol))))) (Math|Rotator|CombineRotators (.rotation _allignoffset) (.rotation (Transformation|GetWorldTransform _propsnapcol))) false true)
          (Actor|Tick|SetActorTickEnabled false)
          (Rendering|SetVisibility (Variables|Default|GetGhost) false false)
          (Variables|Default|SetbAttached true)
          (CallFunction|OnSnap true (Actor|GetParentActor (Components|GetOwner _propsnapcol)))
          (Class|BPIProps|SnapDispatchCall(Message) (Variables|Default|GetPropSnap) true)
          (return bAttach self)))
      (Transformation|DetachFromComponent _staticmesh "KeepWorld" "KeepWorld" "KeepWorld" false)
      (Physics|SetSimulatePhysics _staticmesh true)
      (goto _label))))

(fn SendParams
  (params (bIn :type Boolean) (NameIn :type Name :default "None") (VecIn :type Vector :default "0, 0, 0") (SC_In :type Scene%20Component%20Object%20Reference) (Actor :type Actor%20Object%20Reference))
  (return false "None" "0, 0, 0" 0 0.0))

(fn SendPropSnapTolerance
  (return "0, 0, 0"))

(fn TrySnap
  (params (PropAllign :type Scene%20Component%20Object%20Reference))
  (return false 0))