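; BP_IA_Oven is an interactable oven actor in the interaction system, with an animated skeletal mesh, a door and a drawer.
; On BeginPlay it attaches Door and Drawer to sockets on the skeletal mesh, keeping their world transforms, so they follow its animation.
; Interact forwards its Param as a name message to the mesh's anim instance, leaving the response to the animation side.
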(event EventBeginPlay
  (bind _skm (Variables|Default|GetSKM))
  (|CallParentFunction)
  (Transformation|AttachComponentToComponent (Variables|Default|GetDoor) _skm "Doors" "KeepWorld" "KeepWorld" "KeepWorld" true)
  (Transformation|AttachComponentToComponent (Variables|Default|GetDrawer) _skm "Drawer1" "KeepWorld" "KeepWorld" "KeepWorld" true))

(event EventTick
  (params (DeltaSeconds :type Float%20%28single-precision%29))
  (|CallParentFunction DeltaSeconds) ; This node is disabled and will not be called.\nDrag off pins to build functionality.
)

(event Collision|EventActorBeginOverlap
  (params (OtherActor :type Actor%20Object%20Reference))
  (|CallParentFunction OtherActor) ; This node is disabled and will not be called.\nDrag off pins to build functionality.
)

(event EventInteract
  (params (Param :type Name :default "None"))
  (Class|BPIInteractions|AMSSendParam(Message) (Components|SkeletalMesh|GetAnimInstance (Variables|Default|GetSKM)) false Param))

(fn ConstructionScript
  (|CallParentFunction))