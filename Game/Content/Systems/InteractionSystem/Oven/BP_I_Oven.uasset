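; BP_I_Oven is an interactable oven in the interaction system, with a door and a drawer.
; On BeginPlay it requests a scene component from its linked actor through SendParamsMessage.
; It attaches Door and Drawer to that component's named sockets, keeping their world transforms.
; Interact passes its parameter straight to ConditionMet; the oven adds no other interaction logic here.
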(event EventBeginPlay
  (|CallParentFunction)
  (bind _sc_response (Class|BPIInteractions|SendParams(Message) (Variables|Default|GetLinkedActor) false "None" "0, 0, 0"))
  (Transformation|AttachComponentToComponent (Variables|Default|GetDoor) _sc_response "Doors" "KeepWorld" "KeepWorld" "KeepWorld" true)
  (Transformation|AttachComponentToComponent (Variables|Default|GetDrawer) _sc_response "Drawer1" "KeepWorld" "KeepWorld" "KeepWorld" true))

(event Collision|EventActorBeginOverlap
  (params (OtherActor :type Actor%20Object%20Reference))
  (|CallParentFunction OtherActor) ; This node is disabled and will not be called.\nDrag off pins to build functionality.
)

(event EventTick
  (params (DeltaSeconds :type Float%20%28single-precision%29))
  (|CallParentFunction DeltaSeconds) ; This node is disabled and will not be called.\nDrag off pins to build functionality.
)

(event EventInteract
  (params (Param :type Name :default "None"))
  (CallFunction|ConditionMet Param))

(fn ConstructionScript
  (|CallParentFunction))