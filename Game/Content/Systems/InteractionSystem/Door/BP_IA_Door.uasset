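; BP_IA_Door is an interactable door that opens and closes by playing sections of AM_Door on its skeletal mesh.
; Interact toggles it with "OC" when unlocked and idle, and clears Locked with "ULCK"; montage notifies commit the Open state, and only opening triggers SFX.
; BeginPlay attaches Open0/Open1 to the door bone and poses initially open doors with a zero-rate montage.
; The construction script mirrors the door via negative X scale when Flipped.
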(event EventBeginPlay
  (bind _skm (Variables|Default|GetSKM))
  (|CallParentFunction)
  (Transformation|AttachComponentToComponent (Variables|Default|GetOpen0) _skm "Bone_001" "KeepWorld" "KeepWorld" "KeepWorld" false)
  (Transformation|AttachComponentToComponent (Variables|Default|GetOpen1) _skm "Bone_001" "KeepWorld" "KeepWorld" "KeepWorld" false)
  (if (Variables|Default|GetbOpen)
    (Animation|Montage|PlayMontage (Variables|Default|GetSKM) "/Game/Systems/InteractionSystem/Door/AM_Door.AM_Door" 0.0 0.0 "Close")))

(event Collision|EventActorBeginOverlap
  (params (OtherActor :type Actor%20Object%20Reference))
  (|CallParentFunction OtherActor) ; This node is disabled and will not be called.\nDrag off pins to build functionality.
)

(event EventTick
  (params (DeltaSeconds :type Float%20%28single-precision%29))
  (|CallParentFunction DeltaSeconds) ; This node is disabled and will not be called.\nDrag off pins to build functionality.
)

(event EventInteract
  (params (Param :type Name :default "None"))
  (bind _skm (Variables|Default|GetSKM))
  (Utilities|IfName Param "OC"
    (:True
      (if (Math|Boolean|NORBoolean (Variables|Default|GetbIsMoving) (Variables|Default|GetbLocked))
        (if (not (Variables|Default|GetbOpen))
          (Class|AudioParameterControllerInterface|SetTriggerParameter (Variables|Default|GetSFX) "Open")
          (bind _notifyname (Animation|Montage|PlayMontage _skm "/Game/Systems/InteractionSystem/Door/AM_Door.AM_Door" 1.0 0.0 "Open")
            (:then
              (Variables|Default|SetbIsMoving true :!label _label))
            (:OnNotifyBegin
              (Utilities|FlowControl|Sequence
                (:then_0
                  (Utilities|IfName _notifyname "O"
                    (:True
                      (Variables|Default|SetbIsMoving false)
                      (Variables|Default|SetbOpen true)))))))
          (else
            (bind _notifyname_2 (Animation|Montage|PlayMontage _skm "/Game/Systems/InteractionSystem/Door/AM_Door.AM_Door" 1.0 0.0 "Close")
              (:then
                (goto _label))
              (:OnNotifyBegin
                (Utilities|FlowControl|Sequence
                  (:then_0
                    (Utilities|IfName _notifyname_2 "O"
                      (:True
                        (Variables|Default|SetbIsMoving false)
                        (Variables|Default|SetbOpen false)))))))))))
    (:False
      (Utilities|IfName Param "ULCK"
        (:True
          (Variables|Default|SetbLocked false))))))

(fn ConstructionScript
  (|CallParentFunction)
  (Transformation|SetRelativeScale3D (Variables|Default|GetBP) (Math|Vector|MakeVector (Math|Float|SelectFloat -1.0 1.0 (Variables|Default|GetbFlipped)) 1.0 1.0)))