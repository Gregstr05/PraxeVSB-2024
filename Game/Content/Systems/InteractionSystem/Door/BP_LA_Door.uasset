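; BP_LA_Door is an animated door in the interaction system, opened and closed by name-based conditions.
; OnConditionMet maps "O" and "C" to OpenClose, which plays sections of AM_Door on the skeletal mesh and messages LinkedInteractor on montage notifies.
; AMSSendParam receives names from the animation Blueprint to disable or enable the collision component.
; SendParams exposes the skeletal mesh to callers.
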(event Custom|OpenClose
  (params (bOpen :type Boolean))
  (bind _linkedinteractor (Variables|Default|GetLinkedInteractor))
  (bind _skm (Variables|Default|GetSKM))
  (if bOpen
    (Animation|Montage|PlayMontage _skm "/Game/Systems/InteractionSystem/Door/AM_Door.AM_Door" 1.0 0.0 "Open"
      (:OnNotifyBegin
        (Class|BPIInteractions|AMSSendParam(Message) _linkedinteractor false "AnimDoneO")))
    (else
      (Animation|Montage|PlayMontage _skm "/Game/Systems/InteractionSystem/Door/AM_Door.AM_Door" 1.0 0.0 "Close"
        (:OnNotifyBegin
          (Class|BPIInteractions|AMSSendParam(Message) _linkedinteractor false "AnimDoneC"))))))

(event EventBeginPlay
  (|CallParentFunction))

(event Collision|EventActorBeginOverlap
  (params (OtherActor :type Actor%20Object%20Reference))
  (|CallParentFunction OtherActor) ; This node is disabled and will not be called.\nDrag off pins to build functionality.
)

(event EventTick
  (params (DeltaSeconds :type Float%20%28single-precision%29))
  (|CallParentFunction DeltaSeconds) ; This node is disabled and will not be called.\nDrag off pins to build functionality.
)

(event EventAMSSendParam
  (params (BoolParam :type Boolean) (NameParam :type Name :default "None"))
  (bind _col (Variables|Default|GetCol))
  ;[0.349 0 0.3344] Based on behavior in ABP recieve event when to enable/disable collision
  (Utilities|FlowControl|Sequence
    (:then_0
      (Utilities|IfName NameParam "C_D"
        (:True
          (Collision|SetCollisionEnabled _col "NoCollision"))))
    (:then_1
      (Utilities|IfName NameParam "C_E"
        (:True
          (Collision|SetCollisionEnabled _col "QueryAndPhysics"))))))

(fn ConstructionScript
  (|CallParentFunction))

(fn OnConditionMet
  (params (Param :type Name :default "None"))
  (Utilities|IfName Param "O"
    (:True
      (CallFunction|OpenClose true))
    (:False
      (Utilities|IfName Param "C"
        (:True
          (CallFunction|OpenClose false))))))

(fn SendParams
  (params (bIn :type Boolean) (NameIn :type Name :default "None") (VecIn :type Vector :default "0, 0, 0") (SC_In :type Scene%20Component%20Object%20Reference) (Actor :type Actor%20Object%20Reference))
  (return false "None" "0, 0, 0" (Variables|Default|GetSKM) 0.0))