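; Interactable door that toggles open and closed by driving a linked animated actor.
; On BeginPlay, it attaches its Open0 and Open1 components to the Bone_001 socket of the component returned by that actor.
; An "OC" interaction fires ConditionMet with "O" or "C" based on the door state and blocks further interaction while moving.
; AnimDone messages received through AMSSendParam update the open state and release the lock.
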(event EventBeginPlay
  (|CallParentFunction)
  (bind _sc_response (Class|BPIInteractions|SendParams(Message) (Variables|Default|GetLinkedActor) false "None" "0, 0, 0"))
  (Transformation|AttachComponentToComponent (Variables|Default|GetOpen0) _sc_response "Bone_001" "KeepWorld" "KeepWorld" "KeepWorld" true)
  (Transformation|AttachComponentToComponent (Variables|Default|GetOpen1) _sc_response "Bone_001" "KeepWorld" "KeepWorld" "KeepWorld" true))

(event Collision|EventActorBeginOverlap
  (params (OtherActor :type Actor%20Object%20Reference))
  (|CallParentFunction OtherActor) ; This node is disabled and will not be called.\nDrag off pins to build functionality.
)

(event EventTick
  (params (DeltaSeconds :type Float%20%28single-precision%29))
  (|CallParentFunction DeltaSeconds))

(event EventAMSSendParam
  (params (BoolParam :type Boolean) (NameParam :type Name :default "None"))
  (Utilities|FlowControl|Sequence
    (:then_0
      (if (== NameParam "AnimDoneO")
        (Variables|Default|SetbDoorOpen true)
        (Variables|Default|SetbIsMoving false :!label _label)))
    (:then_1
      (if (== NameParam "AnimDoneC")
        (Variables|Default|SetbDoorOpen false)
        (goto _label)))))

(event EventInteract
  (params (Param :type Name :default "None"))
  (if (and (not (Variables|Default|GetbIsMoving)) (== Param "OC"))
    (if (Variables|Default|GetbDoorOpen)
      (CallFunction|ConditionMet "C")
      (else
        (CallFunction|ConditionMet "O")))
    (Variables|Default|SetbIsMoving true)))

(fn ConstructionScript
  (|CallParentFunction))