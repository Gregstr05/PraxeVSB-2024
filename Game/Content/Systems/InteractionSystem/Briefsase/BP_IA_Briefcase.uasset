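; BP_IA_Briefcase is an interactable briefcase actor that opens and closes when interacted with.
; Its Interact event responds only when the name parameter is "OC", using a FlipFlop to alternate between the two states.
; Each state plays the "Open" or "Close" section of a single montage, AM_Briefcase, on the skeletal mesh.
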(event EventBeginPlay
  (|CallParentFunction) ; This node is disabled and will not be called.\nDrag off pins to build functionality.
)

(event Collision|EventActorBeginOverlap
  (params (OtherActor :type Actor%20Object%20Reference))
  (|CallParentFunction OtherActor) ; This node is disabled and will not be called.\nDrag off pins to build functionality.
)

(event EventTick
  (params (DeltaSeconds :type Float%20%28single-precision%29))
  (|CallParentFunction DeltaSeconds) ; This node is disabled and will not be called.\nDrag off pins to build functionality.
)

(event EventInteract
  (params (Param :type Name :default "None"))
  (bind _skm (Variables|Default|GetSKM))
  (Utilities|IfName Param "OC"
    (:True
      (Utilities|FlowControl|FlipFlop
        (:A
          (Animation|Montage|PlayMontage _skm "/Game/Systems/InteractionSystem/Briefsase/AM_Briefcase.AM_Briefcase" 1.0 0.0 "Open"))
        (:B
          (Animation|Montage|PlayMontage _skm "/Game/Systems/InteractionSystem/Briefsase/AM_Briefcase.AM_Briefcase" 1.0 0.0 "Close"))))))

(fn ConstructionScript
  (|CallParentFunction))