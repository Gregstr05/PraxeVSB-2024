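; BP_IA_DoorReader is a card reader that unlocks a linked door when a component tagged with its UnlockParam enters ReadCol.
; It detaches the card from the player, snaps it to the reader's socket and plays a swipe montage with sound.
; On blend out, or via ForceUnlock, it messages the door and mirror reader "ULCK" and shows Open; receiving "ULCK" only updates visuals.
; Construction sets the Locked visuals and card color.
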(event OnComponentBeginOverlap(ReadCol)
  (params (OverlappedComponent :type Primitive%20Component%20Object%20Reference) (OtherActor :type Actor%20Object%20Reference) (OtherComp :type Primitive%20Component%20Object%20Reference) (OtherBodyIndex :type Integer) (bFromSweep :type Boolean) (SweepResult :type Hit%20Result%20Structure%20%28by%20ref%29))
  (if (Components|ComponentHasTag OtherComp (Variables|Default|GetUnlockParam))
    (Class|BPIInteractions|Interact(Message) (Game|Player|GetPlayerPawn 0) "Detach")
    (Physics|SetSimulatePhysics OtherComp false)
    (Transformation|AttachComponentToComponent OtherComp (Variables|Default|GetSKM) "CardSnap" "SnapToTarget" "SnapToTarget" "KeepWorld" false)
    (Transformation|SetRelativeRotation OtherComp "0.000000,180.000000,90.000000" false false)
    (Animation|Montage|PlayMontage (Variables|Default|GetSKM) "/Game/Systems/InteractionSystem/DoorCardReader/ReadCard.ReadCard" 0.7 0.0 "Start"
      (:then
        (Audio|Components|Audio|Play (Variables|Default|GetSFX) 0.0))
      (:OnBlendOut
        (Physics|SetSimulatePhysics OtherComp true)
        (Class|BPIInteractions|Interact(Message) (Variables|Default|GetDoorToUnlock) "ULCK")
        (Rendering|SetVisibility (Variables|Default|GetClosed) false false)
        (Rendering|SetVisibility (Variables|Default|GetOpen) true false)
        (Class|BPIInteractions|Interact(Message) (Variables|Default|GetMirrorReader) "ULCK")))))

(event Custom|ForceUnlock
  (Class|BPIInteractions|Interact(Message) (Variables|Default|GetDoorToUnlock) "ULCK")
  (Rendering|SetVisibility (Variables|Default|GetClosed) false false)
  (Rendering|SetVisibility (Variables|Default|GetOpen) true false)
  (Class|BPIInteractions|Interact(Message) (Variables|Default|GetMirrorReader) "ULCK"))

(event EventBeginPlay
  (|CallParentFunction) ; This node is disabled and will not be called.\nDrag off pins to build functionality.
)

(event Collision|EventActorBeginOverlap
  (params (OtherActor :type Actor%20Object%20Reference))
  (|CallParentFunction OtherActor) ; This node is disabled and will not be called.\nDrag off pins to build functionality.
)

(event EventTick
  (params (DeltaSeconds :type Float%20%28single-precision%29))
  (|CallParentFunction DeltaSeconds) ; This node is disabled and will not be called.\nDrag off pins to build functionality.
)

(event EventInteract
  (params (Param :type Name :default "None"))
  (Utilities|IfName Param "ULCK"
    (:True
      (Rendering|SetVisibility (Variables|Default|GetClosed) false false)
      (Rendering|SetVisibility (Variables|Default|GetOpen) true false))))

(fn ConstructionScript
  (bind _blocked (Variables|Default|GetbLocked))
  (|CallParentFunction)
  (Rendering|SetVisibility (Variables|Default|GetClosed) _blocked false)
  (Rendering|SetVisibility (Variables|Default|GetOpen) (not _blocked) false)
  (bind _returnvalue (Rendering|Material|CreateDynamicMaterialInstance "/Game/Systems/PropSystem/Props/KeyCard/MI_DoorReader.MI_DoorReader" "None" "None" :!class /Script/Engine.KismetMaterialLibrary))
  (Rendering|Material|SetMaterial (Variables|Default|GetSKM) 0 _returnvalue)
  (Rendering|Material|SetVectorParameterValue _returnvalue "CardColor" (Variables|Default|GetCardColor) :!class /Script/Engine.MaterialInstanceDynamic))