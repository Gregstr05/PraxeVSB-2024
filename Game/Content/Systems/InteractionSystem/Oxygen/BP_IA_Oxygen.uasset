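; Oxygen station interactable: a repair puzzle where eleven knobs must match randomized targets before the unit can be switched on.
; BeginPlay spawns an OxyCard snap point and randomizes targets, knob positions and color assignments, pre-solving if already Functioning.
; Knob turns wrap within a fixed range, drive AnimSKM and report tolerance matches to the card, which can query targets by color.
; Pressing BR with all knobs matched turns it on and fires OnFixed.
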(event Custom|TurnOn
  (Rendering|SetVisibility (Variables|Default|GetOff) false false)
  (Rendering|SetVisibility (Variables|Default|GetOn) true false))

(event EventBeginPlay
  (bind _returnvalue (Transformation|GetActorTransform))
  (bind (_location _rotation _scale) (Math|Transform|BreakTransform _returnvalue))
  (bind _returnvalue_2 (Game|SpawnActorfromClass "/Game/Systems/PropSystem/BP_PropSnap.BP_PropSnap_C" (Math|Transform|MakeTransform (Math|Vector|MakeVector (+ (.x _location) -25.0) (.y _location) (+ (.z _location) 1.2e+02)) (Math|Rotator|MakeRotator (.roll _rotation) (.pitch _rotation) 9e+01) _scale) "Undefined" "MultiplyWithRoot" self 0))
  (Variables|/Game/Systems/PropSystem/BP_PropSnap.BP_PropSnap_C|SetSnapParam _returnvalue_2 "OxyCard")
  (Variables|/Game/Systems/PropSystem/BP_PropSnap.BP_PropSnap_C|SetTolerance _returnvalue_2 "30.000000,30.000000,30.000000")
  (Variables|/Game/Systems/PropSystem/BP_PropSnap.BP_PropSnap_C|SetSnapColSize _returnvalue_2 1e+01)
  (|CallParentFunction)
  (Class|BPIInteractions|Interact(Message) _returnvalue_2 "OxyCard")
  (CallFunction|Initialize))

(event Collision|EventActorBeginOverlap
  (params (OtherActor :type Actor%20Object%20Reference))
  (|CallParentFunction OtherActor) ; This node is disabled and will not be called.\nDrag off pins to build functionality.
)

(event EventTick
  (params (DeltaSeconds :type Float%20%28single-precision%29))
  (|CallParentFunction DeltaSeconds) ; This node is disabled and will not be called.\nDrag off pins to build functionality.
)

(event EventDynamicInteract
  (params (Param :type Name :default "None") (X :type Float%20%28double-precision%29) (Y :type Float%20%28double-precision%29))
  (bind _knobstates (Variables|Default|GetKnobStates))
  (bind _knobsfinishstates (Variables|Default|GetKnobsFinishStates))
  (bind _tocomplete (Variables|Default|GetToComplete))
  (bind _value (Utilities|Map|Find _knobstates Param))
  (bind _value_2 (Utilities|Map|Find _tocomplete Param))
  (bind _returnvalue (+ _value_2 0.1))
  (bind _returnvalue_2 (- _value_2 0.1))
  (bind _returnvalue_3 (+ _value X))
  (bind _returnvalue_4 (<= _returnvalue_3 0.0))
  (bind _returnvalue_5 (+ _returnvalue_3 2.0))
  (bind _returnvalue_6 (>= _returnvalue_3 2.0))
  (bind _returnvalue_7 (- _returnvalue_3 2.0))
  (bind _returnvalue_8 (Math|Float|SelectFloat _returnvalue_7 _returnvalue_3 _returnvalue_6))
  (bind _returnvalue_9 (Math|Float|SelectFloat _returnvalue_5 _returnvalue_3 _returnvalue_4))
  (bind _returnvalue_10 (Math|Float|SelectFloat _returnvalue_8 _returnvalue_9 _returnvalue_6))
  (bind _returnvalue_11 (> _returnvalue_10 _returnvalue_2))
  (bind _returnvalue_12 (< _returnvalue_10 _returnvalue))
  (bind _returnvalue_13 (and _returnvalue_12 _returnvalue_11))
  (Utilities|IfName Param "Stick"
    (:True
      (Class|BPIInteractions|DynamicInteract(Message) (Variables|Default|GetAnimSKM) Param X Y))
    (:False
      (Utilities|Map|Add _knobstates Param _returnvalue_10)
      (Class|BPIInteractions|DynamicInteract(Message) (Variables|Default|GetAnimSKM) Param _returnvalue_10 0.0)
      (Utilities|DualifDoOnce _returnvalue_13
        (:True
          (Utilities|Map|Add _knobsfinishstates Param true))
        (:False
          (Utilities|Map|Remove _knobsfinishstates Param)))
      (Class|BPIInteractions|AMSSendParam(Message) (Variables|Default|GetOxyCard) _returnvalue_13 Param))))

(event EventInteract
  (params (Param :type Name :default "None"))
  (bind _knobstates (Variables|Default|GetKnobStates))
  (Class|BPIInteractions|AMSSendParam(Message) (Variables|Default|GetAnimSKM) false Param)
  (Utilities|IfName Param "A"
    (:True
      (bind _keys (Utilities|Map|Keys _knobstates))
      (for _array_element _keys
        (Class|BPIInteractions|AMSSendParam(Message) (Variables|Default|GetOxyCard) (and (< (.Value (Utilities|Map|Find _knobstates _array_element)) (+ (.Value (Utilities|Map|Find (Variables|Default|GetToComplete) _array_element)) 0.1)) (> (.Value (Utilities|Map|Find _knobstates _array_element)) (- (.Value (Utilities|Map|Find (Variables|Default|GetToComplete) _array_element)) 0.1))) _array_element)
        (if (and (< (.Value (Utilities|Map|Find _knobstates _array_element)) (+ (.Value (Utilities|Map|Find (Variables|Default|GetToComplete) _array_element)) 0.1)) (> (.Value (Utilities|Map|Find _knobstates _array_element)) (- (.Value (Utilities|Map|Find (Variables|Default|GetToComplete) _array_element)) 0.1)))
          (Utilities|Map|Add (Variables|Default|GetKnobsFinishStates) _array_element true))))
    (:False
      (Utilities|IfName Param "BR"
        (:True
          (if (and (>= (Utilities|Map|Length (Variables|Default|GetKnobsFinishStates)) 11) (not (Variables|Default|GetbFunctioning)))
            (CallFunction|Turnon)
            (Default|CallOnFixed)
            (Variables|Default|SetbFunctioning true)))))))

(event EventSetActor
  (params (Actor :type Actor%20Object%20Reference) (Param :type Name :default "None"))
  (Variables|Default|SetOxyCard Actor))

(fn ConstructionScript
  (|CallParentFunction))

(fn SendParams
  (params (bIn :type Boolean) (NameIn :type Name :default "None") (VecIn :type Vector :default "0, 0, 0") (SC_In :type Scene%20Component%20Object%20Reference) (Actor :type Actor%20Object%20Reference))
  (return false "None" "0, 0, 0" 0 0.0))

(fn Initialize
  (bind _bfunctioning (Variables|Default|GetbFunctioning))
  (bind _knobstates (Variables|Default|GetKnobStates))
  (Utilities|Array|Shuffle (Variables|Default|GetKnobCollors))
  (bind _array (CallFunction|RandomizedFloatArray 11 0.0 2.0))
  (for _index (range 0 10)
    (Utilities|Map|Add (Variables|Default|GetToComplete) (Utilities|String|StringToName (Utilities|String|Append "B" (Utilities|String|ToString(Integer) _index))) (Utilities|Array|Get(acopy) _array _index))
    (Utilities|Map|Add _knobstates (Utilities|String|StringToName (Utilities|String|Append "B" (Utilities|String|ToString(Integer) _index))) (Math|Float|SelectFloat (Utilities|Array|Get(acopy) _array _index) (Math|Random|RandomFloatinRange 0.0 2.0) _bfunctioning))
    (Class|BPIInteractions|DynamicInteract(Message) (Variables|Default|GetAnimSKM) (Utilities|String|StringToName (Utilities|String|Append "B" (Utilities|String|ToString(Integer) _index))) (.Value (Utilities|Map|Find _knobstates (Utilities|String|StringToName (Utilities|String|Append "B" (Utilities|String|ToString(Integer) _index))))) 0.0))
  (Utilities|FlowControl|Sequence
    (:then_0
      (if _bfunctioning
        (CallFunction|Turnon)))
    (:then_1
      (return))))

(fn SendCardData
  (params (KnobsParam :type Name :default "None"))
  (bind _arr (LocalVariables|GetArr))
  (for (_array_element _array_index) (Variables|Default|GetKnobCollors)
    (if (== _array_element KnobsParam)
      (Utilities|Map|Add _arr (Utilities|String|StringToName (Utilities|String|Append "B" (Utilities|String|ToString(Integer) _array_index))) (.Value (Utilities|Map|Find (Variables|Default|GetToComplete) (Utilities|String|StringToName (Utilities|String|Append "B" (Utilities|String|ToString(Integer) _array_index))))))))
  (return _arr))