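; Interactable ladder actor that moves the first-person character up or down and plays a level sequence for the climb.
; Interact checks its name param for GoUp or GoDown, then has the player controller possess the Pawn reference.
; It then teleports the character to the TpUp or TpDown transform and plays the matching LSUp or LSDown sequence.
; Handing control back to the character is not done in this Blueprint.
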(event EventBeginPlay
  (|CallParentFunction) ; This node is disabled and will not be called.\nDrag off pins to build functionality.
)

(event Collision|EventActorBeginOverlap
  (params (OtherActor :type Actor%20Object%20Reference))
  (|CallParentFunction OtherActor) ; This node is disabled and will not be called.\nDrag off pins to build functionality.
)

(event EventTick
  (params (DeltaSeconds :type Float%20%28single-precision%29))
  (|CallParentFunction DeltaSeconds) ; This node is disabled and will not be called.\nDrag off pins to build functionality.
)

(event EventInteract
  (params (Param :type Name :default "None"))
  (Utilities|FlowControl|Sequence
    (:then_0
      (Utilities|IfName Param "GoDown"
        (:True
          (bind _returnvalue (Actor|GetActorOfClass "/Game/FirstPerson/Blueprints/BP_FirstPersonCharacter.BP_FirstPersonCharacter_C"))
          (Utilities|FlowControl|Sequence
            (:then_0
              (Pawn|Possess (Game|GetPlayerController 0) (Variables|Default|GetPawn) :!label _label))
            (:then_1
              (Transformation|SetActorTransform _returnvalue (Transformation|GetWorldTransform (Variables|Default|GetTpDown)) false true)
              (Sequencer|Player|Play (Variables|/Script/LevelSequence.LevelSequenceActor|GetSequencePlayer (Variables|Default|GetLS_Down)) :!class /Script/MovieScene.MovieSceneSequencePlayer))))
        (:False
          (Utilities|IfName Param "GoUp"
            (:True
              (bind _returnvalue_2 (Actor|GetActorOfClass "/Game/FirstPerson/Blueprints/BP_FirstPersonCharacter.BP_FirstPersonCharacter_C"))
              (Utilities|FlowControl|Sequence
                (:then_0
                  (goto _label))
                (:then_1
                  (Transformation|SetActorTransform _returnvalue_2 (Transformation|GetWorldTransform (Variables|Default|GetTpUp)) false true)
                  (Sequencer|Player|Play (Variables|/Script/LevelSequence.LevelSequenceActor|GetSequencePlayer (Variables|Default|GetLS_Up)) :!class /Script/MovieScene.MovieSceneSequencePlayer))))))))))

(fn ConstructionScript
  (|CallParentFunction))

(fn SendParams
  (params (bIn :type Boolean) (NameIn :type Name :default "None") (VecIn :type Vector :default "0, 0, 0") (SC_In :type Scene%20Component%20Object%20Reference) (Actor :type Actor%20Object%20Reference))
  (return false "None" "0, 0, 0" 0 0.0))