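; BP_IA_Locker is an interactable locker in the interaction system that toggles between open and closed.
; Its Interact event responds only to the "OC" name parameter, starting the SFX audio and alternating through a FlipFlop.
; Each branch fires the matching Open or Close audio trigger parameter and plays that section of the AM_Locker montage on the skeletal mesh.
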(event EventBeginPlay
  (|CallParentFunction) ; This node is disabled and will not be called.\nDrag off pins to build functionality.
)

(event Collision|EventActorBeginOverlap
  (params (OtherActor :type Actor%20Object%20Reference))
  (|CallParentFunction OtherActor) ; This node is disabled and will not be called.\nDrag off pins to build functionality.
)

(event EventTick
  (params (DeltaSeconds :type Float%20%28single-precision%29))
  (|CallParentFunction DeltaSeconds) ; This node is disabled and will not be called.\nDrag off pins to build functionality.
)

(event EventInteract
  (params (Param :type Name :default "None"))
  (bind _skm (Variables|Default|GetSKM))
  (bind _sfx (Variables|Default|GetSFX))
  (Utilities|IfName Param "OC"
    (:True
      (Audio|Components|Audio|Play _sfx 0.0)
      (Utilities|FlowControl|FlipFlop
        (:A
          (Class|AudioParameterControllerInterface|SetTriggerParameter _sfx "Open")
          (Animation|Montage|PlayMontage _skm "/Game/Systems/InteractionSystem/Locker/AM_Locker.AM_Locker" 1.0 0.0 "Open"))
        (:B
          (Class|AudioParameterControllerInterface|SetTriggerParameter _sfx "Close")
          (Animation|Montage|PlayMontage _skm "/Game/Systems/InteractionSystem/Locker/AM_Locker.AM_Locker" 1.0 0.0 "Close"))))))

(fn ConstructionScript
  (|CallParentFunction))