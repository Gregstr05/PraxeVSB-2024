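; Interactable toilet Blueprint that lets the cover and seat be raised and lowered separately by interaction.
; On BeginPlay it attaches Seat and Cover to matching sockets on a component returned by the linked actor.
; Interact uses the hit part's name and a three-state value (closed, cover open, fully open) to choose the ConditionMet trigger.
; A moving flag blocks further input until an AnimDone message arrives.
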(event EventBeginPlay
  (|CallParentFunction)
  (bind _sc_response (Class|BPIInteractions|SendParams(Message) (Variables|Default|GetLinkedActor) false "None" "0, 0, 0"))
  (Transformation|AttachComponentToComponent (Variables|Default|GetSeat) _sc_response "Seat" "KeepWorld" "KeepWorld" "KeepWorld" true)
  (Transformation|AttachComponentToComponent (Variables|Default|GetCover) _sc_response "Cover" "KeepWorld" "KeepWorld" "KeepWorld" true))

(event Collision|EventActorBeginOverlap
  (params (OtherActor :type Actor%20Object%20Reference))
  (|CallParentFunction OtherActor) ; This node is disabled and will not be called.\nDrag off pins to build functionality.
)

(event EventTick
  (params (DeltaSeconds :type Float%20%28single-precision%29))
  (|CallParentFunction DeltaSeconds) ; This node is disabled and will not be called.\nDrag off pins to build functionality.
)

(event EventInteract
  (params (Param :type Name :default "None"))
  (if (not (Variables|Default|GetbIsMoving))
    (Utilities|IfName Param "Cover"
      (:True
        (switch int (Variables|Default|GetState)
          (:0
            (CallFunction|ConditionMet "Open" :!label _label)
            (Variables|Default|SetState 1))
          (:1
            (CallFunction|ConditionMet "Close" :!label _label_2)
            (Variables|Default|SetState 0))
          (:2
            (goto _label_2))))
      (:False
        (Utilities|IfName Param "Seat"
          (:True
            (switch int (Variables|Default|GetState)
              (:0
                _)
              (:1
                _)
              (:2
                (goto _label)))
            (CallFunction|ConditionMet "OpenF")
            (Variables|Default|SetState 2)))))
    (Variables|Default|SetbIsMoving true)))

(event EventAMSSendParam
  (params (BoolParam :type Boolean) (NameParam :type Name :default "None"))
  (if (== NameParam "AnimDone")
    (Variables|Default|SetbIsMoving false)))

(fn ConstructionScript
  (|CallParentFunction))