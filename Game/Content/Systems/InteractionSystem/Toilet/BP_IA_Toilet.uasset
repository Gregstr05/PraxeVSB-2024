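; BP_IA_Toilet is an interactable toilet whose cover and seat open and close through skeletal mesh animation.
; BeginPlay attaches both parts to SKM sockets, keeping world transforms.
; Interact uses the "Cover" or "Seat" name to advance a three-state machine, sending Open, Close or OpenF messages to the anim instance.
; IsMoving blocks further interaction until an "AnimDone" message returns through AMSSendParam.
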(event EventBeginPlay
  (bind _skm (Variables|Default|GetSKM))
  (|CallParentFunction)
  (Transformation|AttachComponentToComponent (Variables|Default|GetSeat) _skm "Seat" "KeepWorld" "KeepWorld" "KeepWorld" true)
  (Transformation|AttachComponentToComponent (Variables|Default|GetCover) _skm "Cover" "KeepWorld" "KeepWorld" "KeepWorld" true))

(event Collision|EventActorBeginOverlap
  (params (OtherActor :type Actor%20Object%20Reference))
  (|CallParentFunction OtherActor) ; This node is disabled and will not be called.\nDrag off pins to build functionality.
)

(event EventTick
  (params (DeltaSeconds :type Float%20%28single-precision%29))
  (|CallParentFunction DeltaSeconds) ; This node is disabled and will not be called.\nDrag off pins to build functionality.
)

(event EventInteract
  (params (Param :type Name :default "None"))
  (bind _skm (Variables|Default|GetSKM))
  (bind _returnvalue (Components|SkeletalMesh|GetAnimInstance _skm))
  (if (not (Variables|Default|GetbIsMoving))
    (Utilities|IfName Param "Cover"
      (:True
        (switch int (Variables|Default|GetState)
          (:0
            (Class|BPIInteractions|AMSSendParam(Message) _returnvalue false "Open" :!label _label)
            (Variables|Default|SetState 1))
          (:1
            (Class|BPIInteractions|AMSSendParam(Message) _returnvalue false "Close" :!label _label_2)
            (Variables|Default|SetState 0))
          (:2
            (goto _label_2))))
      (:False
        (Utilities|IfName Param "Seat"
          (:True
            (switch int (Variables|Default|GetState)
              (:0
                _)
              (:1
                _)
              (:2
                (goto _label)))
            (Class|BPIInteractions|AMSSendParam(Message) _returnvalue false "OpenF")
            (Variables|Default|SetState 2)))))
    (Variables|Default|SetbIsMoving true)))

(event EventAMSSendParam
  (params (BoolParam :type Boolean) (NameParam :type Name :default "None"))
  (Utilities|IfName NameParam "AnimDone"
    (:True
      (Variables|Default|SetbIsMoving false))))

(fn ConstructionScript
  (|CallParentFunction))