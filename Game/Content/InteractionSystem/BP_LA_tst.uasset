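; BP_LA_tst is an interaction system Blueprint, apparently a test asset, that turns a point light green when a condition is met.
; It overrides OnConditionMet, calls the parent implementation, then sets the PointLight color.
; The event graph holds only disabled default events, and the construction script only calls its parent.
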(event EventBeginPlay
  (|CallParentFunction) ; This node is disabled and will not be called.\nDrag off pins to build functionality.
)

(event Collision|EventActorBeginOverlap
  (params (OtherActor :type Actor%20Object%20Reference))
  (|CallParentFunction OtherActor) ; This node is disabled and will not be called.\nDrag off pins to build functionality.
)

(event EventTick
  (params (DeltaSeconds :type Float%20%28single-precision%29))
  (|CallParentFunction DeltaSeconds) ; This node is disabled and will not be called.\nDrag off pins to build functionality.
)

(fn ConstructionScript
  (|CallParentFunction))

(fn OnConditionMet
  (params (Param :type Name :default "None"))
  (|CallParentFunction Param)
  (Rendering|Components|Light|SetLightColor (Variables|Default|GetPointLight) "(R=0.089607,G=1.000000,B=0.000000,A=1.000000)" true))