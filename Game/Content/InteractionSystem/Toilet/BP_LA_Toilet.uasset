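; Toilet actor for the interaction system that animates its skeletal mesh in response to met conditions.
; OnConditionMet checks its parameter for "Open", "Close" or "OpenF" and forwards the matching name to the SKM anim instance through AMSSendParamMessage.
; The Blueprint holds no animation logic of its own, leaving playback to the anim instance, and its event graph is unused.
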(event EventBeginPlay
  (|CallParentFunction) ; This node is disabled and will not be called.\nDrag off pins to build functionality.
)

(event Collision|EventActorBeginOverlap
  (params (OtherActor :type Actor%20Object%20Reference))
  (|CallParentFunction OtherActor) ; This node is disabled and will not be called.\nDrag off pins to build functionality.
)

(event EventTick
  (params (DeltaSeconds :type Float%20%28single-precision%29))
  (|CallParentFunction DeltaSeconds) ; This node is disabled and will not be called.\nDrag off pins to build functionality.
)

(fn ConstructionScript
  (|CallParentFunction))

(fn OnConditionMet
  (params (Param :type Name :default "None"))
  (bind _skm (Variables|Default|GetSKM))
  (bind _returnvalue (Components|SkeletalMesh|GetAnimInstance _skm))
  (Utilities|FlowControl|Sequence
    (:then_0
      (if (== Param "Open")
        (Class|BPIInteractions|AMSSendParam(Message) _returnvalue false "Open")))
    (:then_1
      (if (== Param "Close")
        (Class|BPIInteractions|AMSSendParam(Message) _returnvalue false "Close")))
    (:then_2
      (if (== Param "OpenF")
        (Class|BPIInteractions|AMSSendParam(Message) _returnvalue false "OpenF")))))