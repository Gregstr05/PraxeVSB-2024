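; BP_I_Toilet is an interactable toilet that steps through three states each time it receives the "Interact" param.
; Successive interactions fire ConditionMet with "Open", "OpenF" and "Close", then wrap back to the first state.
; An IsMoving flag blocks further input after each step until AMSSendParam reports "AnimDone".
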(event EventBeginPlay
  (|CallParentFunction) ; This node is disabled and will not be called.\nDrag off pins to build functionality.
)

(event Collision|EventActorBeginOverlap
  (params (OtherActor :type Actor%20Object%20Reference))
  (|CallParentFunction OtherActor) ; This node is disabled and will not be called.\nDrag off pins to build functionality.
)

(event EventTick
  (params (DeltaSeconds :type Float%20%28single-precision%29))
  (|CallParentFunction DeltaSeconds) ; This node is disabled and will not be called.\nDrag off pins to build functionality.
)

(event EventInteract
  (params (Param :type Name :default "None"))
  (if (and (not (Variables|Default|GetbIsMoving)) (== Param "Interact"))
    (if (== (Variables|Default|GetState) 0)
      (Math|Integer|IncrementInt (Variables|Default|GetState)
        (:%20%20
          (CallFunction|ConditionMet "Open")
          (Variables|Default|SetbIsMoving true :!label _label)))
      (elif (== (Variables|Default|GetState) 1)
        (Math|Integer|IncrementInt (Variables|Default|GetState)
          (:%20%20
            (CallFunction|ConditionMet "OpenF")
            (goto _label)))
        (elif (== (Variables|Default|GetState) 2)
          (Variables|Default|SetState 0)
          (CallFunction|ConditionMet "Close")
          (goto _label))))))

(event EventAMSSendParam
  (params (BoolParam :type Boolean) (NameParam :type Name :default "None"))
  (if (== NameParam "AnimDone")
    (Variables|Default|SetbIsMoving false)))

(fn ConstructionScript
  (|CallParentFunction))