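; Interaction trigger for a door, showing an Open/Close text prompt while the player is inside its box, which is sized by a Size variable.
; Player detection uses named messages that also return the component the text turns to face, with Tick enabled on entry and disabled on exit.
; Interact calls ConditionMet to open or close and hides the prompt until an animation-done message updates the state, text and color.
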(event OnComponentBeginOverlap(Box)
  (params (OverlappedComponent :type Primitive%20Component%20Object%20Reference) (OtherActor :type Actor%20Object%20Reference) (OtherComp :type Primitive%20Component%20Object%20Reference) (OtherBodyIndex :type Integer) (bFromSweep :type Boolean) (SweepResult :type Hit%20Result%20Structure%20%28by%20ref%29))
  (bind (_bboolresponse _nameresponse _vecresponce _sc_response) (Class|BPIInteractions|SendParams(Message) OtherActor false "DoorText" "0, 0, 0"))
  (if (== _nameresponse "Player")
    (Variables|Default|SetbPlayerInside true)
    (if (not (Variables|Default|GetbIsMoving))
      (Rendering|SetVisibility (Variables|Default|GetTextRender) true false)
      (Actor|Tick|SetActorTickEnabled true)
      (Variables|Default|SetTarget _sc_response))))

(event OnComponentEndOverlap(Box)
  (params (OverlappedComponent :type Primitive%20Component%20Object%20Reference) (OtherActor :type Actor%20Object%20Reference) (OtherComp :type Primitive%20Component%20Object%20Reference) (OtherBodyIndex :type Integer))
  (bind _nameresponse (Class|BPIInteractions|SendParams(Message) OtherActor false "DoorText" "0, 0, 0"))
  (if (== _nameresponse "Player")
    (Variables|Default|SetbPlayerInside false)
    (Rendering|SetVisibility (Variables|Default|GetTextRender) false false)
    (Actor|Tick|SetActorTickEnabled false)
    (Variables|Default|SetTarget 0)))

(event EventBeginPlay
  (|CallParentFunction) ; This node is disabled and will not be called.\nDrag off pins to build functionality.
)

(event Collision|EventActorBeginOverlap
  (params (OtherActor :type Actor%20Object%20Reference))
  (|CallParentFunction OtherActor) ; This node is disabled and will not be called.\nDrag off pins to build functionality.
)

(event EventTick
  (params (DeltaSeconds :type Float%20%28single-precision%29))
  (bind _textrender (Variables|Default|GetTextRender))
  (bind _target (Variables|Default|GetTarget))
  (|CallParentFunction DeltaSeconds)
  (Utilities|IsValid _target
    (:Is%20Valid
      (Transformation|SetWorldRotation _textrender (Math|Rotator|FindLookatRotation (Transformation|GetWorldLocation _textrender) (Transformation|GetWorldLocation _target)) false false))))

(event EventAMSSendParam
  (params (BoolParam :type Boolean) (NameParam :type Name :default "None"))
  (bind _textrender (Variables|Default|GetTextRender))
  (Utilities|FlowControl|Sequence
    (:then_0
      (if (== NameParam "AnimDoneO")
        (Variables|Default|SetbDoorOpen true)
        (Rendering|Components|TextRender|SetText _textrender (Utilities|Text|MakeLiteralText "Close"))
        (Rendering|Components|TextRender|SetTextRenderColor _textrender (Math|Color|MakeColor 0 0 255 255))
        (Variables|Default|SetbIsMoving false :!label _label)
        (if (Variables|Default|GetbPlayerInside)
          (Rendering|SetVisibility _textrender true false))))
    (:then_1
      (if (== NameParam "AnimDoneC")
        (Variables|Default|SetbDoorOpen false)
        (Rendering|Components|TextRender|SetText _textrender (Utilities|Text|MakeLiteralText "Open"))
        (Rendering|Components|TextRender|SetTextRenderColor _textrender (Math|Color|MakeColor 55 178 55 255))
        (goto _label)))))

(event EventInteract
  (params (Param :type Name :default "None"))
  (if (== Param "Interact")
    (if (Variables|Default|GetbDoorOpen)
      (CallFunction|ConditionMet "C")
      (else
        (CallFunction|ConditionMet "O")))
    (Rendering|SetVisibility (Variables|Default|GetTextRender) false false)
    (Variables|Default|SetbIsMoving true)))

(fn ConstructionScript
  (bind _box (Variables|Default|GetBox))
  (|CallParentFunction)
  (Components|Box|SetBoxExtent _box (Variables|Default|GetSize) true)
  (Transformation|AddLocalOffset _box (Math|Vector|MakeVector 0.0 0.0 (.z (Variables|Default|GetSize))) false true))