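; Interactable door Blueprint that drives its skeletal mesh's open and close animation when an interaction condition is met.
; It overrides OnConditionMet, letting the parent class evaluate the condition and return an "O" or "C" result.
; That result is sent to the mesh's AnimInstance as a true or false bool through AMSSendParamMessage, leaving the animation itself to the AnimBP.
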(event EventBeginPlay
  (|CallParentFunction))

(event Collision|EventActorBeginOverlap
  (params (OtherActor :type Actor%20Object%20Reference))
  (|CallParentFunction OtherActor) ; This node is disabled and will not be called.\nDrag off pins to build functionality.
)

(event EventTick
  (params (DeltaSeconds :type Float%20%28single-precision%29))
  (|CallParentFunction DeltaSeconds) ; This node is disabled and will not be called.\nDrag off pins to build functionality.
)

(fn ConstructionScript
  (|CallParentFunction))

(fn OnConditionMet
  (params (Param :type Name :default "None"))
  (bind _skm (Variables|Default|GetSKM))
  (bind _returnvalue (Components|SkeletalMesh|GetAnimInstance _skm))
  (bind _outparam (|CallParentFunction Param))
  (if (== _outparam "O")
    (Class|BPIInteractions|AMSSendParam(Message) _returnvalue true "None")
    (return _outparam)
    (elif (== _outparam "C")
      (Class|BPIInteractions|AMSSendParam(Message) _returnvalue false "None")
      (return _outparam))))