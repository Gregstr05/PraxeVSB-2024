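; Interactable submarine periscope that lets the player take control of a separate periscope pawn.
; Unlock, called on BeginPlay, enables query collision on the interaction component, then plays the working animation once while a timeline slides the skeletal mesh along Z.
; A "Periscope" interaction stores the current player pawn on the periscope pawn, then has the player controller possess it.
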(event Custom|Unlock
  (Collision|SetCollisionEnabled (Variables|Default|GetInteract_0) "QueryOnly")
  (Utilities|FlowControl|DoOnce false
    (:Completed
      (Components|Animation|PlayAnimation (Variables|Default|GetSKM) "/Game/Submarine/Periscope/Mesh/periskop_Working_Anim.periskop_Working_Anim" false)
      (bind _height (Timeline|Periscope Play)
        (:Update
          (Transformation|SetRelativeLocation (Variables|Default|GetSKM) (* "0.000000,0.000000,-221.209201" _height) false false))))))

(event EventBeginPlay
  (CallFunction|Unlock))

(event Collision|EventActorBeginOverlap
  (params (OtherActor :type Actor%20Object%20Reference)))

(event EventTick
  (params (DeltaSeconds :type Float%20%28single-precision%29)))

(event EventInteract
  (params (Param :type Name :default "None"))
  (bind _periscopepawn (Variables|Default|GetPeriscopePawn))
  (Utilities|IfName Param "Periscope"
    (:True
      (Variables|/Game/Submarine/Periscope/BP_Periscope_ext.BP_Periscope_ext_C|SetPlayerPawn _periscopepawn (Game|Player|GetPlayerPawn 0))
      (Pawn|Possess (Game|GetPlayerController 0) _periscopepawn))))

(fn ConstructionScript)