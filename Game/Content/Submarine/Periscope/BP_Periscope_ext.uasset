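; BP_Periscope_ext is a possessable submarine periscope that the player looks through and turns horizontally.
; Possession creates the overlay widget once and adds it to the viewport, and unpossession removes it.
; Look input plays a Rotation timeline that adds relative yaw scaled by horizontal input, with debug prints of input and yaw.
; The interact input returns control to the stored player pawn.
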(event Input|EnhancedActionEvents|EnhancedInputActionIA_Look
  (params (ActionValue :type Vector%202D%20Structure) (ElapsedSeconds :type Float%20%28double-precision%29) (TriggeredSeconds :type Float%20%28double-precision%29) (InputAction :type Input%20Action%20Object%20Reference :default "/Game/FirstPerson/Input/Actions/IA_Look.IA_Look"))
  (bind _periscope (Variables|Default|GetPeriscope))
  (Development|PrintString (Utilities|String|ToString(Vector2d) ActionValue) true true "(R=1.000000,G=0.000000,B=0.677049,A=1.000000)" 2.0 "Coords")
  (bind _newtrack_0 (Timeline|Rotation Play)
    (:Update
      (Transformation|AddRelativeRotation _periscope (Math|Rotator|MakeRotator 0.0 0.0 (* _newtrack_0 (/ (.X (Math|Vector2D|BreakVector2D ActionValue)) 2.0))) false false)
      (Development|PrintString (Utilities|String|ToString(Float) (.yaw (Variables|/Script/Engine.SceneComponent|GetRelativeRotation _periscope))) true true "(R=0.000000,G=0.660000,B=1.000000,A=1.000000)" 2.0 "Rotation"))))

(event Input|EnhancedActionEvents|EnhancedInputActionIA_Interract
  (params (ActionValue :type Boolean) (ElapsedSeconds :type Float%20%28double-precision%29) (TriggeredSeconds :type Float%20%28double-precision%29) (InputAction :type Input%20Action%20Object%20Reference :default "/Game/ThirdPerson/Input/Actions/IA_Interract.IA_Interract"))
  (:Started
    (Pawn|Possess (Game|GetPlayerController 0) (Variables|Default|GetPlayerPawn))))

(event EventPossessed
  (params (NewController :type Controller%20Object%20Reference))
  (Utilities|IsValid (Variables|Default|GetViewOverlay)
    (:Is%20Valid
      _)
    (:Is%20Not%20Valid
      (bind _returnvalue (UserInterface|CreateWidget "/Game/Submarine/Periscope/WBP_Periscope_Overlay.WBP_Periscope_Overlay_C"))
      (bind _output_get (Variables|Default|SetViewOverlay _returnvalue))))
  (UserInterface|Viewport|AddtoViewport _output_get 0))

(event EventUnpossessed
  (params (OldController :type Controller%20Object%20Reference))
  (Widget|RemovefromParent (Variables|Default|GetViewOverlay)))

(fn ConstructionScript)