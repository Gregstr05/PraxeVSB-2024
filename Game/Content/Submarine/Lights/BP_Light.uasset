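; BP_Light is a configurable light fixture for the submarine that appears as either a wall or ceiling light.
; Its construction script shows the wall mesh (SvetloStena) or ceiling mesh (SvetloStrop) and their children based on IsWallMounted.
; One Color variable tints both point lights and both meshes' EmissiveColor material parameter, keeping glow and illumination matched.
; The event graph holds no runtime logic.
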(event EventBeginPlay)

(event Collision|EventActorBeginOverlap
  (params (OtherActor :type Actor%20Object%20Reference)))

(event EventTick
  (params (DeltaSeconds :type Float%20%28single-precision%29)))

(fn ConstructionScript
  (bind _iswallmounted (Variables|Default|GetIsWallMounted))
  (bind _color (Variables|Default|GetColor))
  (Rendering|SetVisibility (Variables|Default|Getsvetlo_stena) _iswallmounted true)
  (Rendering|SetVisibility (Variables|Default|Getsvetlo_strop) (not _iswallmounted) true)
  (Rendering|Components|Light|SetLightColor (Variables|Default|GetPointLight1) _color true)
  (Rendering|Material|SetVectorParameterValueonMaterials (Variables|Default|Getsvetlo_strop) "EmissiveColor" (Math|Conversions|ToVector(LinearColor) _color)))