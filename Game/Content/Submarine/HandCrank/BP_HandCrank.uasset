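; Hand crank actor for the submarine that the player turns through a dynamic interaction to build up a progress value.
; When the "Crank" interaction reports X and Y input that both pass a small threshold and differ, the mesh rotates a fixed step.
; Each step also raises Progress slightly until it reaches full, printing it for debugging.
; Nothing here consumes Progress, and a mouse-position capture is left unconnected.
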(event EventBeginPlay)

(event Collision|EventActorBeginOverlap
  (params (OtherActor :type Actor%20Object%20Reference)))

(event EventTick
  (params (DeltaSeconds :type Float%20%28single-precision%29)))

(event EventDynamicInteract
  (params (Param :type Name :default "None") (X :type Float%20%28double-precision%29) (Y :type Float%20%28double-precision%29))
  (Utilities|IfName Param "Crank"
    (:True
      (if (and (and (>= (Math|Float|Absolute(Float) X) 0.05) (>= (Math|Float|Absolute(Float) Y) 0.05)) (!= X Y))
        (if (< (Variables|Default|Getprogress) 1.0)
          (Transformation|AddLocalRotation (Variables|Default|GetSM_HandCrank) "0.000000,5.000000,0.000000" false false)
          (bind _output_get (Variables|Default|Setprogress (+ (Variables|Default|Getprogress) 0.001)))
          (Development|PrintString (Utilities|String|ToString(Float) _output_get) true true "(R=1.000000,G=0.000000,B=0.861698,A=1.000000)" 2.0 "Progress"))))))

(fn ConstructionScript)